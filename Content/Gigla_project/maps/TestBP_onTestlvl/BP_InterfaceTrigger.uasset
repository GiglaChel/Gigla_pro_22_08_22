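; Test trigger actor that switches a referenced ActorToInteract on and off through interface-style ActivateMessage and DeactivateMessage calls.
; Its Box component activates the target on begin overlap and deactivates it on end overlap, with no actor filter, printing whether each call succeeded.
; On BeginPlay it also binds to the player MainCharacter's OnDamage, where a FlipFlop alternates activation and deactivation on each hit.
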(event OnComponentBeginOverlap(Box)
  (params (OverlappedComponent :type Primitive%20Component%20Object%20Reference) (OtherActor :type Actor%20Object%20Reference) (OtherComp :type Primitive%20Component%20Object%20Reference) (OtherBodyIndex :type Integer) (bFromSweep :type Boolean) (SweepResult :type Hit%20Result%20Structure%20%28by%20ref%29))
  (bind _success (Class|BPIActivation|Activate(Message) (Variables|Default|GetActorToInteract)))
  (if _success
    (Development|PrintString "activated")
    (else
      (Development|PrintString "activ fail"))))

(event OnComponentEndOverlap(Box)
  (params (OverlappedComponent :type Primitive%20Component%20Object%20Reference) (OtherActor :type Actor%20Object%20Reference) (OtherComp :type Primitive%20Component%20Object%20Reference) (OtherBodyIndex :type Integer))
  (bind _success (Class|BPIActivation|Deactivate(Message) (Variables|Default|GetActorToInteract)))
  (if _success
    (Development|PrintString "Desctivated")
    (else
      (Development|PrintString "Deact fail"))))

(event Custom|OnDamage
  (params (NewHealth :type Float%20%28double-precision%29))
  (Development|PrintString "Interfacetriger_Active" true true "(R=0.546875,G=0.456087,B=0.029705,A=1.000000)")
  (Utilities|FlowControl|FlipFlop
    (:A
      (Class|BPIActivation|Activate(Message) (Variables|Default|GetActorToInteract)))
    (:B
      (Class|BPIActivation|Deactivate(Message) (Variables|Default|GetActorToInteract)))))

(event EventBeginPlay
  (bind _asmain_character (Utilities|Casting|CastToMainCharacter (Game|GetPlayerCharacter 0)))
  (EventDispatchers|AssignOnDamage _asmain_character (delegate Custom|OnDamage)))

(fn ConstructionScript)