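; BP_BoxPlatform is a drop-off platform that takes the box a MainCharacter is carrying.
; When the character begins overlapping its Box component, it stores the carried box, clears the character's reference, detaches the box and moves it just above the platform's origin.
; Debug strings report a successful placement, an empty-handed character or an overlap by another actor.
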(event OnComponentBeginOverlap(Box)
  (params (OverlappedComponent :type Primitive%20Component%20Object%20Reference) (OtherActor :type Actor%20Object%20Reference) (OtherComp :type Primitive%20Component%20Object%20Reference) (OtherBodyIndex :type Integer) (bFromSweep :type Boolean) (SweepResult :type Hit%20Result%20Structure%20%28by%20ref%29))
  (bind _asmain_character (Utilities|Casting|CastToMainCharacter OtherActor)
    (:then
      (Utilities|IsValid (Variables|/Game/Gigla_project/Characters/MainCharacter.MainCharacter_C|GetCurrentBoxCarrying _asmain_character)
        (:Is%20Valid
          (Variables|Default|SetBox%20on%20platform (Variables|/Game/Gigla_project/Characters/MainCharacter.MainCharacter_C|GetCurrentBoxCarrying _asmain_character))
          (Variables|/Game/Gigla_project/Characters/MainCharacter.MainCharacter_C|SetCurrentBoxCarrying _asmain_character 0)
          (Transformation|DetachFromActor (Variables|Default|GetBox%20on%20platform) "KeepRelative" "KeepRelative" "KeepRelative")
          (Transformation|SetActorLocation (Variables|Default|GetBox%20on%20platform) (+ (Transformation|GetActorLocation) "0.000000,0.000000,50.000000") false false)
          (Development|PrintString "Box Plased"))
        (:Is%20Not%20Valid
          (Development|PrintString "No Box in character"))))
    (:CastFailed
      (Development|PrintString "Hello"))))

(fn ConstructionScript)